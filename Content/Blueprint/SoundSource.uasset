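; SoundSource is an actor that remotely controls playback of a numbered sound source through a TCP connection actor (Bp_tcp), found at BeginPlay.
; Beginning an overlap sends a play-start command with SourceNo and position, and ending one sends play-stop, without filtering the overlapping actor.
; While sound is on, Tick sends a position update whenever the source's location in player 0's local space changes, so player rotation also counts.
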(event EventBeginPlay
  ;[1 1 1] 開始時にネットワーク接続クラスのオブジェクト取得
  (bind _returnvalue (Actor|GetActorOfClass "/Game/Blueprint/bp_tcp.bp_tcp_C")))

(event Collision|EventActorBeginOverlap
  (params (OtherActor :type Actor%20Object%20Reference))
  ;[1 1 1] 範囲内に入ったら、再生開始コマンドを送信する。再生信号のソース番号と再生開始時の位置座標が必要となる。
  (Variables|Default|SetSoundOn true)
  (Development|PrintString "Begin Overlap")
  (bind _returnvalue (Default|SendPlayStart (stale EventBeginPlay _returnvalue) (Variables|Default|GetSourceNo) (Math|Transform|InverseTransformLocation (Transformation|GetActorTransform (Game|GetPlayerCharacter 0)) (Transformation|GetActorLocation))))
  (if _returnvalue
    (Development|PrintString "Send Play Start")
    (else
      (Development|PrintString "Error: Send Play Start"))))

(event EventTick
  (params (DeltaSeconds :type Float%20%28single-precision%29))
  (bind _returnvalue (Transformation|GetActorLocation))
  (bind _returnvalue_2 (Game|GetPlayerCharacter 0))
  (bind _returnvalue_3 (Transformation|GetActorTransform _returnvalue_2))
  (bind _returnvalue_4 (Math|Transform|InverseTransformLocation _returnvalue_3 _returnvalue))
  ;[1 1 1] 範囲内で移動を検知したら、位置を更新する
  (if (Variables|Default|GetSoundOn)
    (if (Utilities|Operators|NotEqual(!=) (Variables|Default|GetPosition) _returnvalue_4 0.0)
      (bind _output_get (Variables|Default|SetPosition _returnvalue_4))
      ;[1 1 1] 範囲内で移動を検知したら、位置情報コマンドを送信する。再生信号のソース番号と再生開始時の位置座標が必要となる。
      (bind _returnvalue_5 (Default|SendPosition (stale EventBeginPlay _returnvalue) (Variables|Default|GetSourceNo) _output_get))
      (if (not _returnvalue_5)
        (Development|PrintString "Error: Send Position")))))

(event Collision|EventActorEndOverlap
  (params (OtherActor :type Actor%20Object%20Reference))
  ;[1 1 1] 範囲外に出たら、再生終了コマンドを送信する。再生信号のソース番号が必要となる。
  (Variables|Default|SetSoundOn false)
  (Development|PrintString "End Overlap")
  (bind _returnvalue (Default|SendPlayStop (stale EventBeginPlay _returnvalue) (Variables|Default|GetSourceNo)))
  (if _returnvalue
    (Development|PrintString "Send Play Stop")
    (else
      (Development|PrintString "Error: Send Play Stop"))))

(fn ConstructionScript)
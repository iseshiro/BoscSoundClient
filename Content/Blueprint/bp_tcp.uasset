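; TCP client Blueprint that sends position and play/stop commands for numbered sources to an external server.
; It connects to a hardcoded LAN address on BeginPlay, stores the connection ID, prints received messages, and disconnects on EndPlay.
; Helper functions for other classes build text commands, scaling positions by 0.01, and pass them to SendMessage, which sends length before payload.
; Starting playback sends the position before the play command.
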(event Custom|Connected
  (params (ConnectionId :type Integer))
  (Variables|Default|SetConnectionId ConnectionId)
  (Variables|Default|SetConnecting true)
  (Development|PrintString "Connected"))

(event Custom|Received
  (params (ConnectionId :type Integer) (Message :type Array%20of%20Bytes))
  (bind _returnvalue (Class|TcpSocketConnection|MessageReadString Message (Utilities|Array|Length Message)))
  (Development|PrintString _returnvalue))

(event Custom|Disconnected
  (params (ConnectionId :type Integer))
  (Variables|Default|SetConnecting false)
  (Development|PrintString "Disconnected"))

(event EventBeginPlay
  (Class|TcpSocketConnection|Connect "192.168.0.5" 2001 (delegate Custom|Disconnected) (delegate Custom|Connected) (delegate Custom|Received)))

(event EventEndPlay
  (params (EndPlayReason :type EEndPlayReason%20Enum :default "Destroyed"))
  (Class|TcpSocketConnection|Disconnect (Variables|Default|GetConnectionId)))

(fn ConstructionScript)

(fn SendMessage
  (params (Message :type String))
  (bind _connectionid (Variables|Default|GetConnectionId))
  (bind _returnvalue (Class|TcpSocketConnection|SendData _connectionid (Class|TcpSocketConnection|ToBytes(Integer) (Utilities|String|Len Message))))
  (if _returnvalue
    (bind _returnvalue_2 (Class|TcpSocketConnection|SendData _connectionid (Class|TcpSocketConnection|ToBytes(String) Message))))
  (return _returnvalue_2))

(fn MakePosition
  (params (SourceNo :type Integer) (Position :type Vector))
  (bind _returnvalue (* Position "0.010000,0.010000,0.010000"))
  (bind (_x _y _z) (Math|Vector|BreakVector _returnvalue))
  (return (Utilities|String|Append "posi " (Utilities|String|ToString(Integer) SourceNo) " " (Utilities|String|ToString(Float) _x) " " (Utilities|String|ToString(Float) _y) " " (Utilities|String|ToString(Float) _z))))

(fn SendPosition
  (params (SourceNo :type Integer) (Position :type Vector))
  (bind _returnvalue (CallFunction|MakePosition 0 SourceNo Position))
  (bind _returnvalue_2 (CallFunction|SendMessage 0 _returnvalue))
  (return _returnvalue_2))

(fn SendPlayStop
  (params (SourceNo :type Integer))
  (bind _returnvalue (CallFunction|SendMessage (Utilities|String|Append "stop " (Utilities|String|ToString(Integer) SourceNo))))
  (return _returnvalue))

(fn SendPlayStart
  (params (SourceNo :type Integer) (Position :type Vector))
  (Development|PrintString "Play Start")
  (CallFunction|SendPosition SourceNo Position)
  (bind _returnvalue (CallFunction|SendMessage (Utilities|String|Append "play " (Utilities|String|ToString(Integer) SourceNo))))
  (Development|PrintString "Send Message in Play")
  (return _returnvalue))